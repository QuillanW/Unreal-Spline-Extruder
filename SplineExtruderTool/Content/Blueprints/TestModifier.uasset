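; Spline Toolkit test modifier that adjusts instantiation rules and passes extrusion rules through unchanged.
; Instantiation spacing shrinks as absolute curvature at the sampled point rises, using a clamped CurvatureMultiplier term scaled by DistanceMultiplier.
; A random roll also adds a "Hook" anchor on some steps, with fixed X and Z offsets and the rule's own Y offset.
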(fn `ModifyExtrusionStep`
  (params (Context :type "SplineToolkitStepContext Structure (by ref)") (InRule :type "SplineToolkitExtrusionRule Structure (by ref)"))
  (returns (ReturnValue :type "SplineToolkitExtrusionRule Structure"))
  (bind _structout (setmembers `SplineToolkitExtrusionRule` :`StructRef` InRule))
  (return _structout))

(fn `ModifyInstantiationStep`
  (params (Context :type "SplineToolkitStepContext Structure (by ref)") (InRule :type "SplineToolkitInstantiationRule Structure (by ref)"))
  (returns (ReturnValue :type "SplineToolkitInstantiationRule Structure"))
  (bind (_mesh _material _overlaymaterial _enabled _spacing _offset _rotationoffset _scale _anchors) (break `SplineToolkitInstantiationRule` InRule))
  (if (> (`KismetMathLibrary.RandomFloatInRange` 0.0 1.0) 0.7)
    (`KismetArrayLibrary.Array_Add` _anchors (make `SplineToolkitAnchor` (`KismetMathLibrary.MakeVector` 450.0 (.y _offset) 638.071025) "Hook")))
  (bind _structout (setmembers `SplineToolkitInstantiationRule` :`StructRef` InRule :`Spacing` (- _spacing (* (`self.Distance Multiplier`) (`KismetMathLibrary.FClamp` (* (`KismetMathLibrary.Abs` (`.Curvature` (break `SplineToolkitRmfSample` (`.RMFSample` (break `SplineToolkitStepContext` Context))))) (`self.Curvature Multiplier`)))))))
  (return _structout))