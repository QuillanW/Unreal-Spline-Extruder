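; Spline Toolkit instantiation modifier that, going by its name, places corner signs only where a spline bends sharply enough.
; ModifyInstantiationStep reads the RMF sample's curvature at each step and enables the rule only when its absolute value exceeds MinCurve.
; The curvature's sign picks the side: positive curvature keeps the rule's Offset, otherwise the whole vector is negated.
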(fn `ModifyInstantiationStep`
  (params (Context :type "SplineToolkitStepContext Structure (by ref)") (InRule :type "SplineToolkitInstantiationRule Structure (by ref)"))
  (returns (ReturnValue :type "SplineToolkitInstantiationRule Structure"))
  (bind (_mesh _material _overlaymaterial _stepprecision _enabled _spacing _offset) (break `SplineToolkitInstantiationRule` InRule))
  (bind (_position _distance _tangent _bitangent _reference _roll _curvature) (break `SplineToolkitRmfSample` (`.RMFSample` (break `SplineToolkitStepContext` Context))))
  (bind _structout (setmembers `SplineToolkitInstantiationRule` :`StructRef` InRule :`Enabled` (> (`KismetMathLibrary.Abs` _curvature) (`self.Min Curve`)) :`Offset` (`KismetMathLibrary.SelectVector` _offset (* _offset -1.0) (> _curvature 0.0)) :`RotationOffset` (struct)))
  (return _structout))